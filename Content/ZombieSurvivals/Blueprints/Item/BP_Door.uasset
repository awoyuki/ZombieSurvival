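; BP_Door is a key-locked sliding door that takes keys from the player on overlap and lights one indicator per key.
; The construction script stacks a light mesh for each required key, and unlocking switches their materials on and plays a sound.
; Once all keys are in, a looping timer interpolates the door sideways and enables an enter zone.
; That zone fires OnPlayerGetOverZone, disables itself and snaps the player to its XY position.
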(event `self.ReceiveBeginPlay`
  (set `self.KeyUnlocked` 0))

(event `self.TriggerBox.OnComponentBeginOverlap`
  (params (OverlappedComponent :type "PrimitiveComponent Object Reference") (OtherActor :type "Actor Object Reference") (OtherComp :type "PrimitiveComponent Object Reference") (OtherBodyIndex :type Integer) (bFromSweep :type Boolean) (SweepResult :type "HitResult Structure (by ref)"))
  (if (`self.ActorHasTag` OtherActor "Player")
    (bind _aszs_player (cast `ZS_Player` OtherActor))
    (bind _returnvalue (`ZS_Player.UseKey` _aszs_player))
    (`self.OnUnlockDoor` _returnvalue)))

(event `OpenDoor`
  (bind _doormesh (`self.DoorMesh`))
  (set `self.DoorOpenLocation` (`KismetMathLibrary.MakeVector` 0.0 (- (.y (`SceneComponent.RelativeLocation` _doormesh)) (* (.y (`SceneComponent.RelativeScale3D` _doormesh)) 100.0))))
  (bind _returnvalue (`KismetSystemLibrary.K2_SetTimer` null "OpenDoorHandling" 0.05 true))
  (set `self.DoorOpenTimerHandle` _returnvalue))

(event `self.EnterZone.OnComponentBeginOverlap`
  (params (OverlappedComponent :type "PrimitiveComponent Object Reference") (OtherActor :type "Actor Object Reference") (OtherComp :type "PrimitiveComponent Object Reference") (OtherBodyIndex :type Integer) (bFromSweep :type Boolean) (SweepResult :type "HitResult Structure (by ref)"))
  (bind _enterzone (`self.EnterZone`))
  (if (`self.ActorHasTag` OtherActor "Player")
    (`PrimitiveComponent.SetCollisionEnabled` _enterzone "NoCollision")
    (`self.OnPlayerGetOverZone`)
    (`self.K2_SetActorLocation` OtherActor (`KismetMathLibrary.MakeVector` (.x (`SceneComponent.K2_GetComponentLocation` _enterzone)) (.y (`SceneComponent.K2_GetComponentLocation` _enterzone)) (.z (`self.K2_GetActorLocation` OtherActor))) false false)))

(fn `OnUnlockDoor`
  (params (NewKey :type Integer))
  (bind _keyrequired (`self.KeyRequired`))
  (if (> NewKey 0)
    (`GameplayStatics.PlaySoundAtLocation` "/Game/ZombieSurvivals/Audio/Common/pickup_key.pickup_key" (`self.K2_GetActorLocation`) (struct) 1.0 1.0 0.0 null null null null))
  (bind _output_get (set `self.KeyUnlocked` (`KismetMathLibrary.Min` (+ NewKey (`self.KeyUnlocked`)) _keyrequired)))
  (`self.UpdateVisualize`)
  (if (>= _output_get _keyrequired)
    (`self.OpenDoor`)
    (`PrimitiveComponent.SetCollisionEnabled` (`self.EnterZone`) "QueryOnly")))

(fn `OpenDoorHandling`
  (`SceneComponent.K2_SetRelativeLocation` (`self.DoorMesh`) (`KismetMathLibrary.VInterpTo` (`SceneComponent.RelativeLocation` (`self.DoorMesh`)) (`self.DoorOpenLocation`) 0.05 10.0) false false))

(fn `UpdateVisualize`
  (for _index (range (`self.KeyUnlocked`))
    (`PrimitiveComponent.SetMaterial` (`|GetArrayItem` (`self.Lights`) _index) 0 "/Game/ZombieSurvivals/Models/Door/Materials/M_DoorLight_On.M_DoorLight_On")))

(fn `UserConstructionScript`
  (for _index (range 1 (+ (`self.KeyRequired`) 1))
    (bind _returnvalue (`AddComponent|NODE_AddStaticMeshComponent-0` :`bManualAttachment` true :`RelativeTransform` (`KismetMathLibrary.MakeTransform` (`KismetMathLibrary.MakeVector` 0.0 0.0 (* _index 40.0)) (struct) (0.5 0.2 0.2))))
    (`StaticMeshComponent.SetStaticMesh` _returnvalue "/Game/ZombieSurvivals/Models/Door/Mesh/SM_Door_Light.SM_Door_Light")
    (`SceneComponent.K2_AttachToComponent` _returnvalue (`self.Light`) "None" "KeepRelative" "KeepRelative" "KeepRelative" true)
    (`KismetArrayLibrary.Array_Add` (`self.Lights`) _returnvalue)))